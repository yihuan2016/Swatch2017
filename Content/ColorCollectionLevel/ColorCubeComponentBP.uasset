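; Colored cube actor for the color collection level that bobs up and down from its spawn location on a timeline.
; The construction script picks blue, yellow, red or a random color from boolean flags, applies it to a dynamic material and stores it as a vector.
; ReturnColorVec3 exposes that vector, and GetNewFromAndTo computes a from/to index pair.
; A Rotate360 yaw-spin timeline exists but never runs.
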(event `self.ReceiveBeginPlay`
  (set `self.InitialLocation` (`self.K2_GetActorLocation`))
  (bind (_direction _z_axis_float) (`Timeline|Move Up and Down`)
    (:`Update`
      (`self.K2_SetActorLocation` (`KismetMathLibrary.MakeVector` (.x (`self.InitialLocation`)) (.y (`self.InitialLocation`)) (+ (.z (`self.InitialLocation`)) _z_axis_float))))))

(fn `GetNewFromAndTo`
  (params (LastIndex :type Integer) (CurrentIndex :type Integer))
  (returns (NewFromIndex :type Integer) (NewToIndex :type Integer))
  (set `self.fNewFrom` 0)
  (set `self.fNewTo` 0)
  (if (== LastIndex CurrentIndex)
    (set `self.fNewFrom` 0)
    (set `self.fNewTo` 1)
    (return (`self.fNewFrom`) (`self.fNewTo`))
    (else
      (set `self.fNewFrom` (+ CurrentIndex 1))
      (if (> LastIndex (`self.fNewFrom`))
        (set `self.fNewTo` 0)
        (return (`self.fNewFrom`) (`self.fNewTo`))
        (else
          (set `self.fNewTo` (+ (`self.fNewFrom`) 1)))))))

(fn `ReturnColorVec3`
  (returns (NewParam :type "Vector Structure"))
  (return (`self.ColorVec3`)))

(fn `UserConstructionScript`
  (bind _returnvalue (`KismetMathLibrary.Conv_ColorToLinearColor` (`self.color`)))
  (bind _returnvalue_2 (`PrimitiveComponent.CreateDynamicMaterialInstance` (`self.Cube`) 0 null))
  (set `self.DynamicMaterial` _returnvalue_2)
  (if (`self.isBlue`)
    (set `self.color` (`KismetMathLibrary.Conv_LinearColorToColor` (`KismetMathLibrary.MakeColor` 0.0 0.14 0.33)))
    (elif (`self.isYellow`)
      (set `self.color` (`KismetMathLibrary.Conv_LinearColorToColor` (`KismetMathLibrary.MakeColor` 1.0 0.85)))
      (elif (`self.isRed`)
        (set `self.color` (`KismetMathLibrary.Conv_LinearColorToColor` (`KismetMathLibrary.MakeColor` 0.85 0.0)))
        (else
          (set `self.color` (`KismetMathLibrary.Conv_LinearColorToColor` (`KismetMathLibrary.MakeColor` (`KismetMathLibrary.RandomFloatInRange` 0.0 1.0) (`KismetMathLibrary.RandomFloatInRange` 0.0 1.0) (`KismetMathLibrary.RandomFloatInRange` 0.0 1.0))))))))
  (`MaterialInstanceDynamic.SetVectorParameterValue` (`self.DynamicMaterial`) "ColorCubeBaseColor" _returnvalue)
  (set `self.ColorVec3` (`KismetMathLibrary.Conv_LinearColorToVector` _returnvalue)))